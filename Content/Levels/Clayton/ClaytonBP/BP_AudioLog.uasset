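; BP_AudioLog is an interactable audio log pickup that plays a recording when the player collects it.
; On activation it plays a backpack pickup sound at its location, calls the KeyCardPickedUp dispatcher, then plays the AudioLog sound in 2D.
; Its interaction functions report an interaction type, mark it as consumable, return no scene info and supply a crosshair pickup prompt.
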(event `self.Activate Scene Object`
  (`GameplayStatics.PlaySoundAtLocation` "/Game/RebelX_Core/Audio/Backpack/SC_Backpack_PickUp.SC_Backpack_PickUp" (`self.K2_GetActorLocation`) (struct) 1.0 1.0 0.0 null null null null)
  (`self.KeyCardPickedUp`)
  (`GameplayStatics.PlaySound2D` (`self.AudioLog`) 1.0 1.0 0.0 null null))

(fn `Get Crosshair Prompt`
  (returns (Prompt :type Text) (Tooltip :type Text))
  (return (`self.Interaction Message`) "[E] Pickup"))

(fn `Get Interaction Type`
  (returns (`Return Value` :type Boolean) (InteractionType :type "/Game/RebelX_Core/Blueprints/Enums/E_InteractionTyoes Enum"))
  (return true "NewEnumerator2"))

(fn `Get Is Consumeable`
  (returns (Consumeable :type Boolean))
  (return true))

(fn `Get Scene Info`
  (returns (`Return Value` :type Boolean))
  (return false))

(fn `UserConstructionScript`
  (`parent.UserConstructionScript`))