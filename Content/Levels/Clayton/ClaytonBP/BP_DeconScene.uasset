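; BP_DeconScene is a one-shot scripted scare scene, triggered when its Box is overlapped.
; It freezes player walking, then plays crane audio from a random offset and a level sequence.
; A timed Delay chain layers camera fades and breathing sounds while repositioning and then destroying the Monster component.
; Finally it restores walk speed and destroys the trigger and crane audio, with no overlap filter or re-entry guard before then.
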(event `self.Box.OnComponentBeginOverlap`
  (params (OverlappedComponent :type "PrimitiveComponent Object Reference") (OtherActor :type "Actor Object Reference") (OtherComp :type "PrimitiveComponent Object Reference") (OtherBodyIndex :type Integer) (bFromSweep :type Boolean) (SweepResult :type "HitResult Structure (by ref)"))
  (set `CharacterMovementComponent.MaxWalkSpeed` 0.0 (`Character.CharacterMovement` (`GameplayStatics.GetPlayerCharacter` 0)))
  (`AudioComponent.Play` (`self.CraneAudio`) (`KismetMathLibrary.RandomFloatInRange` 0.0 26.3))
  (`MovieSceneSequencePlayer.Play` (`LevelSequenceActor.SequencePlayer` (`self.Sequence`)))
  (`KismetSystemLibrary.Delay` 10.0)
  (`PlayerCameraManager.StartCameraFade` :`self` (`GameplayStatics.GetPlayerCameraManager` 0) :`ToAlpha` 10.0 :`Duration` 2.0)
  (`KismetSystemLibrary.Delay` 1.5)
  (`GameplayStatics.PlaySound2D` "/Game/RebelX_Core/Audio/FX/SC_FX_CombatEnded.SC_FX_CombatEnded" 1.0 1.0 0.0 null null)
  (`SceneComponent.K2_SetRelativeLocation` (`self.Monster`) (-500.0 100.0 -150.0) false false)
  (`GameplayStatics.PlaySound2D` "/Game/Levels/Clayton/Audio/Ambient/Breath_shortMonstyer_Cue.Breath_shortMonstyer_Cue" 1.0 1.0 0.0 null null)
  (`KismetSystemLibrary.Delay` 3.0)
  (`PlayerCameraManager.StartCameraFade` :`self` (`GameplayStatics.GetPlayerCameraManager` 0) :`ToAlpha` 10.0 :`Duration` 2.0)
  (`KismetSystemLibrary.Delay` 1.0)
  (`SceneComponent.K2_SetRelativeLocation` (`self.Monster`) (0.0 0.0 -300.0) false false)
  (`ActorComponent.K2_DestroyComponent` (`self.Monster`))
  (`GameplayStatics.PlaySound2D` "/Game/Levels/Clayton/Audio/Ambient/BreathlONGcUE.BreathlONGcUE" 1.0 1.0 0.0 null null)
  (`KismetSystemLibrary.Delay` 10.0)
  (set `CharacterMovementComponent.MaxWalkSpeed` 600.0 (`Character.CharacterMovement` (`GameplayStatics.GetPlayerCharacter` 0)))
  (`ActorComponent.K2_DestroyComponent` (`self.Box`))
  (`ActorComponent.K2_DestroyComponent` (`self.CraneAudio`)))

(fn `UserConstructionScript`)