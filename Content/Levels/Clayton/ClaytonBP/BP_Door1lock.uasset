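; BP_Door1lock is a one-shot scripted door scare in the Clayton level, fired when anything begins overlapping its DoorLock component.
; The overlap rotates the Scene component, plays a door-closing sound, moves DoorLock away and repositions the Monster component with a breath cue.
; After timed delays it starts a player camera fade, moves the Monster down, destroys both Monster and DoorLock, and plays a longer breath sound.
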(event `self.Door Lock.OnComponentBeginOverlap`
  (params (OverlappedComponent :type "PrimitiveComponent Object Reference") (OtherActor :type "Actor Object Reference") (OtherComp :type "PrimitiveComponent Object Reference") (OtherBodyIndex :type Integer) (bFromSweep :type Boolean) (SweepResult :type "HitResult Structure (by ref)"))
  (`SceneComponent.K2_SetRelativeRotation` (`self.Scene`) (`KismetMathLibrary.MakeRotator` 0.0 0.0 100.0) false false)
  (`GameplayStatics.PlaySound2D` "/Game/BlockingStarterPack/Blueprints/AutomaticDoor/Sounds/BigDoor_Closing01.BigDoor_Closing01" 5.0 1.0 0.0 null null)
  (`SceneComponent.K2_SetRelativeLocation` (`self.Door Lock`) (0.0 0.0 300.0) false false)
  (`SceneComponent.K2_SetRelativeLocation` (`self.Monster`) (100.0 60.0 0.0) false false)
  (`GameplayStatics.PlaySound2D` "/Game/Levels/Clayton/Audio/Ambient/Breath_shortMonstyer_Cue.Breath_shortMonstyer_Cue" 1.0 1.0 0.0 null null)
  (`KismetSystemLibrary.Delay` 2.5)
  (`PlayerCameraManager.StartCameraFade` :`self` (`GameplayStatics.GetPlayerCameraManager` 0) :`ToAlpha` 10.0 :`Duration` 2.0)
  (`KismetSystemLibrary.Delay` 1.0)
  (`SceneComponent.K2_SetRelativeLocation` (`self.Monster`) (0.0 0.0 -300.0) false false)
  (`ActorComponent.K2_DestroyComponent` (`self.Monster`))
  (`ActorComponent.K2_DestroyComponent` (`self.Door Lock`))
  (`GameplayStatics.PlaySound2D` "/Game/Levels/Clayton/Audio/Ambient/BreathlONGcUE.BreathlONGcUE" 1.0 1.0 0.0 null null))

(fn `UserConstructionScript`
  (`parent.UserConstructionScript`))