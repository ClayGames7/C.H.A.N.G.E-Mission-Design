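; BP_LadderClimb is an interactable button that, when Retriggerable, teleports the player between placed points, apparently standing in for ladder climbing.
; Interaction interface functions supply its type and crosshair prompt and mark it non-consumable.
; ActivateSceneObject passes a DoOnce, fires the ButtonPressed dispatcher and turns the light green.
; If Retriggerable, it waits briefly, turns yellow, teleports to TP1 then immediately TP2, and resets the gate.
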(event `self.ReceiveTick`
  (params (DeltaSeconds :type "Float (single-precision)")))

(event `self.Activate Scene Object`
  (`/Engine/EditorBlueprintResources/StandardMacros.DoOnce` false :!label _label
    (:`Completed`
      (`self.ButtonPressed`)
      (`LightComponent.SetLightColor` (`self.PointLight`) (struct :`G` 1.0 :`A` 1.0) true)
      (if (`self.bRetriggerable`)
        (`KismetSystemLibrary.Delay` 0.5)
        (`LightComponent.SetLightColor` (`self.PointLight`) (struct :`R` 1.0 :`G` 1.0 :`A` 1.0) true)
        (`self.K2_TeleportTo` :`self` (`GameplayStatics.GetPlayerCharacter` 0) :`DestLocation` (`self.K2_GetActorLocation` (`self.TP_1`)))
        (`self.K2_TeleportTo` :`self` (`GameplayStatics.GetPlayerCharacter` 0) :`DestLocation` (`self.K2_GetActorLocation` (`self.TP_2`)))
        (goto _label :!via `Reset`)))))

(event `self.Attempt Consume Interactable`)

(fn `Get Crosshair Prompt`
  (returns (Prompt :type Text) (Tooltip :type Text))
  (return (`self.Interaction Message`) "[E] INTERACT"))

(fn `Get Interaction Type`
  (returns (`Return Value` :type Boolean) (InteractionType :type "/Game/RebelX_Core/Blueprints/Enums/E_InteractionTyoes Enum"))
  (return true "NewEnumerator2"))

(fn `Get Is Consumeable`
  (returns (Consumeable :type Boolean))
  (return false))

(fn `UserConstructionScript`)