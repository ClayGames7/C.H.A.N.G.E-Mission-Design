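; Interactable keypad scene object for the Clayton level that fires once and broadcasts ButtonPressed on activation.
; Activation turns its point light green; if Retriggerable, the light returns to red after a delay, then a level sequence plays with a click sound and input is disabled.
; The LeverDown timeline then plays cable-snap audio and re-enables input on its updates.
; A HUD objective update for Research Lab 7 is left unwired.
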(event `self.ReceiveTick`
  (params (DeltaSeconds :type "Float (single-precision)")))

(event `self.Activate Scene Object`
  (`/Engine/EditorBlueprintResources/StandardMacros.DoOnce` false
    (:`Completed`
      (`self.ButtonPressed`)
      (`LightComponent.SetLightColor` (`self.PointLight`) (struct :`G` 1.0 :`A` 1.0) true)
      (if (`self.bRetriggerable`)
        (`KismetSystemLibrary.Delay` 1.0)
        (`LightComponent.SetLightColor` (`self.PointLight`) (struct :`R` 1.0 :`G` 0.029223 :`A` 1.0) true)
        (`MovieSceneSequencePlayer.Play` (`LevelSequenceActor.SequencePlayer` (`self.Sequence`)))
        (`GameplayStatics.PlaySoundAtLocation` "/Engine/VREditor/Sounds/UI/Click_on_Button.Click_on_Button" (`self.K2_GetActorLocation`) (struct) 1.0 1.0 0.0 null null null null)
        (`self.DisableInput` null)
        (`KismetSystemLibrary.Delay` 1.0)
        (`Timeline|LeverDown`
          (:`Update`
            (`GameplayStatics.PlaySoundAtLocation` "/Game/RX_C_Bailey_Content/Sounds/CableSnap.CableSnap" (`self.K2_GetActorLocation`) (struct) 1.0 1.0 0.0 null null null null)
            (`self.EnableInput` null)))))))

(fn `Get Crosshair Prompt`
  (returns (Prompt :type Text) (Tooltip :type Text))
  (return (`self.Interaction Message`) "[E] INTERACT"))

(fn `Get Interaction Type`
  (returns (`Return Value` :type Boolean) (InteractionType :type "/Game/RebelX_Core/Blueprints/Enums/E_InteractionTyoes Enum"))
  (return true "NewEnumerator2"))

(fn `Get Is Consumeable`
  (returns (Consumeable :type Boolean))
  (return false))

(fn `UserConstructionScript`)